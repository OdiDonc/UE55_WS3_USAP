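; Actor component that steers its owner along a BP_TargetSpline, optionally auto-selecting the one nearest a forward aim point at BeginPlay.
; Each tick it sets the destination to the spline point closest to that aim point ahead of the owner, a look-ahead path-following technique.
; Pawns receive movement input toward it; other actors move along local X and rotate to face it.
; Debug spheres show both points.
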(event `self.ReceiveBeginPlay`
  (if (`self.AutoFindSpline`)
    (bind _outactors (`GameplayStatics.GetAllActorsOfClass` "/Game/Game/BluePrint/BP_TargetSpline.BP_TargetSpline_C"))
    (bind _asbp_target_spline (cast `/Game/Game/BluePrint/BP_TargetSpline` (`.ReturnValue` (`GameplayStatics.FindNearestActor` (`self.GetForwardAimLocation`) _outactors))))
    (set `self.Target Spline` _asbp_target_spline)))

(event `self.ReceiveTick`
  (params (DeltaSeconds :type "Float (single-precision)"))
  (`self.Update Destination`)
  (`self.Proceed to Destination` DeltaSeconds)
  (`self.Uptade Debug`))

(fn `GetForwardAimLocation`
  (returns (`Front Location` :type "Vector Structure"))
  (bind _returnvalue (`self.GetOwner`))
  (return (+ (`Actor.K2_GetActorLocation` _returnvalue) (* (`Actor.GetActorForwardVector` _returnvalue) (`self.ForwardAimDistance`)))))

(fn `Proceed to Destination`
  (params (`Delta Time` :type "Float (double-precision)"))
  (bind _returnvalue (`self.GetOwner`))
  (bind _returnvalue_2 (`self.GetOwner`))
  (bind _rootcomponent (`Actor.RootComponent` _returnvalue))
  (set `self.Time Since Last Uptade` `Delta Time`)
  (bind _aspawn (cast `Pawn` _returnvalue_2)
    (:`then`
      (`Pawn.AddMovementInput` _aspawn (`KismetMathLibrary.GetForwardVector` (`KismetMathLibrary.FindLookAtRotation` (`SceneComponent.K2_GetComponentLocation` (`Actor.RootComponent` _returnvalue_2)) (`self.Destination`))) (`self.Speed`) false))
    (:`CastFailed`
      (`Actor.K2_AddActorLocalOffset` _returnvalue (`KismetMathLibrary.MakeVector` (* (* (`self.Speed`) (`self.Max Speed cm/s`)) (`self.Time Since Last Uptade`))) false false)
      (`SceneComponent.K2_SetWorldRotation` _rootcomponent (`KismetMathLibrary.FindLookAtRotation` (`SceneComponent.K2_GetComponentLocation` _rootcomponent) (`self.Destination`)) false false))))

(fn `Update Destination`
  (set `self.Destination` (`SplineComponent.FindLocationClosestToWorldLocation` (`/Game/Game/BluePrint/BP_TargetSpline.SplinePath` (`self.Target Spline`)) (`self.GetForwardAimLocation`) "World")))

(fn `Uptade Debug`
  (`KismetSystemLibrary.DrawDebugSphere` (`self.Destination`) 120.0 12 (struct :`R` 1.0 :`G` 0.093222 :`B` 0.083274 :`A` 1.0))
  (`KismetSystemLibrary.DrawDebugSphere` (`self.GetForwardAimLocation`) 120.0 12 (struct :`R` 0.443878 :`G` 0.1072 :`B` 1.0 :`A` 1.0)))