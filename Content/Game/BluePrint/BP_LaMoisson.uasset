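; BP_LaMoisson is an actor that teleports back to its starting location when its capsule overlaps the Roomba teleport box actor.
; On BeginPlay it saves that location, caches BP_BoxTpRoomba's box and registers itself with all BPI_Distribute actors.
; Separate events receive the car and teleport-box references.
; A visibility trace runs while the car is valid, but its result is unused; Tours is an empty stub.
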(event `self.ReceiveBeginPlay`
  (set `self.Tp_Lap` (`SceneComponent.K2_GetComponentLocation` (`self.DefaultSceneRoot`)))
  (bind _returnvalue (`GameplayStatics.GetActorOfClass` "/Game/Game/BluePrint/BP_BoxTpRoomba.BP_BoxTpRoomba_C"))
  (bind _asbp_box_tp_roomba (cast `/Game/Game/BluePrint/BP_BoxTpRoomba` _returnvalue))
  (set `self.Box` (`/Game/Game/BluePrint/BP_BoxTpRoomba.Box` _asbp_box_tp_roomba))
  (bind _outactors (`GameplayStatics.GetAllActorsWithInterface` "/Game/Game/BluePrint/BPI_Distribute.BPI_Distribute_C"))
  (for _array_element _outactors
    (`KismetArrayLibrary.Array_Add` (`self.BPI_Distribute_Actors`) _array_element)
    (message `/Game/Game/BluePrint/BPI_Distribute.Distribute_MoissonVariable` (`self.BPI_Distribute_Actors`) self)))

(event `self.ReceiveTick`
  (params (DeltaSeconds :type "Float (single-precision)"))
  (`/Engine/EditorBlueprintResources/StandardMacros.IsValid` (stale `/Game/Game/BluePrint/BPI_Distribute.Distriubte_VoitureVariable` _output_get) :!label _label
    (:`Is Valid`
      (bind _outhit (`KismetSystemLibrary.LineTraceSingle` (0.0 0.0 0.0) (0.0 0.0 0.0) "TraceTypeQuery1")))))

(event `/Game/Game/BluePrint/BPI_Distribute.Distriubte_VoitureVariable`
  (params (BP_Voiture :type "/Game/Game/BluePrint/BP_Voiture_ Object Reference"))
  (bind _output_get (set `self.BP Voiture` BP_Voiture))
  (goto _label))

(event `self.Capsule.OnComponentBeginOverlap`
  (params (OverlappedComponent :type "PrimitiveComponent Object Reference") (OtherActor :type "Actor Object Reference") (OtherComp :type "PrimitiveComponent Object Reference") (OtherBodyIndex :type Integer) (bFromSweep :type Boolean) (SweepResult :type "HitResult Structure (by ref)"))
  (if (== OtherActor (`self.Box TPRoomba`))
    (`self.K2_SetActorLocation` (`self.Tp_Lap`) false true)))

(event `/Game/Game/BluePrint/BPI_Distribute.BoxTPRoomba`
  (params (BoxTPRoomba :type "/Game/Game/BluePrint/BP_BoxTpRoomba Object Reference"))
  (set `self.Box TPRoomba` BoxTPRoomba))

(fn `Tours`
  (return))

(fn `UserConstructionScript`)