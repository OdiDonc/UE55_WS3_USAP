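; BP_ProjectileLum is a physics projectile that launches relative to the BP_Voiture car, lights up, then destroys itself.
; On BeginPlay it applies an impulse along the inverted hit normal of a car-to-projectile trace.
; The Intensity timeline starts after a delay, or when a gated Tick trace toward the car reports a short hit distance.
; The timeline drives the PointLight and a vertical force scaled by world height, destroying the actor when finished.
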(event `self.ReceiveTick`
  (params (DeltaSeconds :type "Float (single-precision)"))
  (`|ExecutionSequence`
    (:`then_0`
      (`/Engine/EditorBlueprintResources/StandardMacros.Gate` true :!label _label
        (:`Exit`
          (if (< (`.Distance` (`GameplayStatics.BreakHitResult` (stale _outhit))) 900.0)
            (bind (_direction _intensity) (`Timeline|Intensity` :!label _label_2)
              (:`Update`
                (`|ExecutionSequence`
                  (:`then_0`
                    (`PrimitiveComponent.AddForce` (`self.HitBox`) (* (`SceneComponent.K2_GetComponentLocation` (`self.HitBox`)) (0.0 0.0 40.0)) "None" true))
                  (:`then_1`
                    (`LightComponent.SetIntensity` (`self.PointLight`) (* _intensity 5000.0)))))
              (:`Finished`
                (`self.K2_DestroyActor`)))))))
    (:`then_1`
      (bind _outhit (`KismetSystemLibrary.LineTraceSingle` (`SceneComponent.K2_GetComponentLocation` (`self.HitBox`)) (`SceneComponent.K2_GetComponentLocation` (`/Game/Game/BluePrint/BP_Voiture.Voiture_` (stale `self.ReceiveBeginPlay` _returnvalue))) "TraceTypeQuery1"))
      (`KismetSystemLibrary.Delay` 1.0)
      (goto _label :!via `Open`))))

(event `self.ReceiveBeginPlay`
  (bind _returnvalue (`GameplayStatics.GetActorOfClass` "/Game/Game/BluePrint/BP_Voiture.BP_Voiture_C"))
  (bind _outhit (`KismetSystemLibrary.LineTraceSingle` (`SceneComponent.K2_GetComponentLocation` (`/Game/Game/BluePrint/BP_Voiture.Voiture_` _returnvalue)) (`SceneComponent.K2_GetComponentLocation` (`self.HitBox`)) "TraceTypeQuery1"))
  (`PrimitiveComponent.AddImpulse` (`self.HitBox`) (+ (* (`.ImpactNormal` (`GameplayStatics.BreakHitResult` _outhit)) -10000.0) (0.0 0.0 100.0)) "None" true)
  (`KismetSystemLibrary.Delay` 4.0)
  (goto _label_2 :!via `PlayFromStart`))

(fn `UserConstructionScript`)