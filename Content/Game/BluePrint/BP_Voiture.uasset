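; Physics-driven player car with headlights that toggle a freeze collision zone, a light cannon, an expanding horn wave and a menu key.
; Enhanced Input drives forward force, timeline-curved steering torque and a dash impulse that notifies BP_DashWall to change collision; gates throttle dash and cannon.
; A per-tick line trace sets InAir, which blocks throttle, switches damping and runs a fall-force timeline.
; Restart or "Killer" overlaps destroy the car, triggering GameMode respawn.
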(event `self.ReceiveBeginPlay`
  (bind _returnvalue (pcsubsystem `EnhancedInputLocalPlayerSubsystem` (`GameplayStatics.GetPlayerController` 0)))
  ;[0.4819 0.7394 1] Set Linear & Angular Damping
  (`PrimitiveComponent.SetLinearDamping` (`self.Voiture_`) (`self.Linear Damping`))
  (`PrimitiveComponent.SetAngularDamping` (`self.Voiture_`) (`self.Angular Damping`))
  (bind _asbp_voiture_game_mode (cast `/Game/Game/BP_VoitureGameMode` (`GameplayStatics.GetGameMode`)))
  (set `/Game/Game/BP_VoitureGameMode.RespawnTransform` (`self.GetTransform`) _asbp_voiture_game_mode)
  ;[0 1 0.06418] Input Local Player
  (`|ExecutionSequence`
    (:`then_0`
      ;[1 0.03079 0] Phares off BeginPlay
      (`PrimitiveComponent.SetCollisionResponseToAllChannels` (`self.FreezPhares`) "ECR_Ignore"))
    (:`then_1`
      (`/Engine/EditorBlueprintResources/StandardMacros.IsValid` _returnvalue
        (:`Is Valid`
          (`EnhancedInputSubsystemInterface.AddMappingContext` _returnvalue "/Game/Game/Input/IM_Voiture.IM_Voiture" 0 (struct)))))))

(event `EnhancedInput|/Game/Game/Input/Phare`
  (params (ActionValue :type Boolean) (ElapsedSeconds :type "Float (double-precision)") (TriggeredSeconds :type "Float (double-precision)") (InputAction :type "InputAction Object Reference" :default "/Game/Game/Input/Phare.Phare"))
  (bind _pharesl (`self.PharesL`))
  (bind _freezphares (`self.FreezPhares`))
  ;[1 0.04241 0] Phares/Freez on/off
  (:`Started`
    (`SceneComponent.ToggleVisibility` _pharesl false)
    (`SceneComponent.ToggleVisibility` (`self.PharesR`) false)
    (`SceneComponent.ToggleVisibility` (`self.PharesL1`) false)
    (`SceneComponent.ToggleVisibility` (`self.PharesR1`) false)
    ;;[1 0.4561 0.4262] à supp (temp)
    (`SceneComponent.ToggleVisibility` (`self.FreezPhares`) false)
    (if (`SceneComponent.IsVisible` _pharesl)
      (`PrimitiveComponent.SetCollisionResponseToAllChannels` _freezphares "ECR_Overlap")
      (else
        (`PrimitiveComponent.SetCollisionResponseToAllChannels` _freezphares "ECR_Ignore")))))

(event `EnhancedInput|/Game/Game/Input/CanonLumiere`
  (params (ActionValue :type Boolean) (ElapsedSeconds :type "Float (double-precision)") (TriggeredSeconds :type "Float (double-precision)") (InputAction :type "InputAction Object Reference" :default "/Game/Game/Input/CanonLumiere.CanonLumiere"))
  ;[1 0.0669 0] Canon Lumiere
  (:`Triggered`
    (`/Engine/EditorBlueprintResources/StandardMacros.Gate` false :!label _label
      (:`Exit`
        (`|SpawnActorFromClass` "/Game/Game/BluePrint/BP_ProjectileLum.BP_ProjectileLum_C" (`KismetMathLibrary.Conv_VectorToTransform` (`SceneComponent.K2_GetComponentLocation` (`self.CanonLumiere`))) "Undefined" "MultiplyWithRoot" null null)
        (`|ExecutionSequence`
          (:`then_0`
            (`KismetSystemLibrary.Delay` 0.1)
            (goto _label :!via `Open`))
          (:`then_1`
            (goto _label :!via `Close`)))))))

(event `EnhancedInput|/Game/Game/Input/Forward_Backward`
  (params (ActionValue :type "Float (double-precision)") (ElapsedSeconds :type "Float (double-precision)") (TriggeredSeconds :type "Float (double-precision)") (InputAction :type "InputAction Object Reference" :default "/Game/Game/Input/Forward_Backward.Forward_Backward"))
  ;[0.133 0.2084 1] Movement Z_Q_S_D
  (:`Triggered`
    (if (not (`self.In air`))
      (`PrimitiveComponent.AddForce` (`self.Voiture_`) (* (* ActionValue (`self.Vitesse Voiture`)) (`SceneComponent.GetForwardVector` (`self.Voiture_`))) "None" true))))

(event `EnhancedInput|/Game/Game/Input/IA_UI`
  (params (ActionValue :type Boolean) (ElapsedSeconds :type "Float (double-precision)") (TriggeredSeconds :type "Float (double-precision)") (InputAction :type "InputAction Object Reference" :default "/Game/Game/Input/IA_UI.IA_UI"))
  ;[1 1 1] UI
  (:`Started`
    (`KismetSystemLibrary.PrintString` "Hello")
    (bind _returnvalue (`|CreateWidget` "/Game/Game/Menu/WBP_Menu.WBP_Menu_C"))
    (`UserWidget.AddToViewport` _returnvalue 0)
    (set `PlayerController.bShowMouseCursor` true (`GameplayStatics.GetPlayerController` 0))))

(event `self.ReceiveDestroyed`
  ;[0.757 1 0.7609] Restart when press R or killed
  (bind _asbp_voiture_game_mode (cast `/Game/Game/BP_VoitureGameMode` (`GameplayStatics.GetGameMode`)))
  (`/Game/Game/BP_VoitureGameMode.RespawnPlayer` _asbp_voiture_game_mode self))

(event `EnhancedInput|/Game/Game/Input/IA_Restart`
  (params (ActionValue :type Boolean) (ElapsedSeconds :type "Float (double-precision)") (TriggeredSeconds :type "Float (double-precision)") (InputAction :type "InputAction Object Reference" :default "/Game/Game/Input/IA_Restart.IA_Restart"))
  ;[0.757 1 0.7609] Restart when press R or killed
  (:`Started`
    (`self.K2_DestroyActor`)))

(event `EnhancedInput|/Game/Game/Input/Left_Right`
  (params (ActionValue :type "Float (double-precision)") (ElapsedSeconds :type "Float (double-precision)") (TriggeredSeconds :type "Float (double-precision)") (InputAction :type "InputAction Object Reference" :default "/Game/Game/Input/Left_Right.Left_Right"))
  ;[0.133 0.2084 1] Movement Z_Q_S_D
  (:`Triggered`
    (if (`self.In air`)
      (bind (_direction _courbe) (`Timeline|CourbeVirage` :!via `Reverse` :!label _label_2)
        (:`Update`
          (`PrimitiveComponent.AddTorqueInDegrees` (`self.Voiture_`) (`KismetMathLibrary.MakeVector` 0.0 0.0 (* (* _courbe (`self.TorqueMax`)) ActionValue)) "None" true)))
      (else
        (goto _label_2))))
  (:`Completed`
    (`|ExecutionSequence`
      (:`then_0`
        (goto _label_2 :!via `Stop`))
      (:`then_1`
        (goto _label_2 :!via `SetNewTime`)))))

(event `self.CollisionBox.OnComponentBeginOverlap`
  (params (OverlappedComponent :type "PrimitiveComponent Object Reference") (OtherActor :type "Actor Object Reference") (OtherComp :type "PrimitiveComponent Object Reference") (OtherBodyIndex :type Integer) (bFromSweep :type Boolean) (SweepResult :type "HitResult Structure (by ref)"))
  ;[1 0.8157 0.5167] Kill Player when overlap Killer
  (`self.Scene`
    (:`then`
      (if (`ActorComponent.ComponentHasTag` OtherComp "Killer")
        (`self.Voiture_`
          (:`then`
            (`self.K2_DestroyActor`))
          (:`else`))))
    (:`else`)))

(event `EnhancedInput|/Game/Game/Input/Klaxon`
  (params (ActionValue :type Boolean) (ElapsedSeconds :type "Float (double-precision)") (TriggeredSeconds :type "Float (double-precision)") (InputAction :type "InputAction Object Reference" :default "/Game/Game/Input/Klaxon.Klaxon"))
  ;[1 0.8746 0.8845] Wave
  (:`Triggered`
    (bind (_direction _wave) (`Timeline|Wave` :!via `PlayFromStart`)
      (:`Update`
        (`SphereComponent.SetSphereRadius` (`self.Klaxon`) (* _wave (`self.WaveRadius`)) true))
      (:`Finished`
        (`SphereComponent.SetSphereRadius` (`self.Klaxon`) 0.0 true)))))

(event `self.ReceiveTick`
  (params (DeltaSeconds :type "Float (single-precision)"))
  (bind _voiture_ (`self.Voiture_`))
  (bind _returnvalue (`SceneComponent.K2_GetComponentLocation` (`self.Voiture_`)))
  ;[0.204 0.3748 1] Movement air_control
  (`|ExecutionSequence`
    (:`then_0`
      ;[1 0.05564 0] LineTrace Trajectoire (à supp (temp))
      (`KismetSystemLibrary.LineTraceSingle` :`Start` (`SceneComponent.K2_GetComponentLocation` (`self.Voiture_`)) :`End` (+ (`SceneComponent.K2_GetComponentLocation` (`self.Voiture_`)) (0.0 10.0 0.0)) :`TraceChannel` "TraceTypeQuery1" :`DrawDebugType` "Persistent"))
    (:`then_1`
      (bind _outhit (`KismetSystemLibrary.LineTraceSingle` :`Start` _returnvalue :`End` (* _returnvalue (1.0 1.0 -1.0)) :`TraceChannel` "TraceTypeQuery1" :`DrawDebugType` "ForOneFrame"))
      (if (> (`.Distance` (`GameplayStatics.BreakHitResult` _outhit)) 80.0)
        (set `self.In air` true)
        (`PrimitiveComponent.SetLinearDamping` _voiture_ (`self.Linear damping in air`))
        (bind (_direction _courberetomber) (`Timeline|CourbeRetomber` :!via `PlayFromStart` :!label _label_3)
          (:`Update`
            (bind _result (`/Engine/EditorBlueprintResources/StandardMacros.NegateFloat` (* _courberetomber 300000.0))
              (:`  `
                (`PrimitiveComponent.AddForce` (`self.Voiture_`) (`KismetMathLibrary.MakeVector` 0.0 0.0 _result) "None" true)))))
        (else
          (set `self.In air` false)
          (`PrimitiveComponent.SetLinearDamping` _voiture_ (`self.Linear Damping`))
          (goto _label_3 :!via `Stop`))))))

(event `EnhancedInput|/Game/Game/Input/Dash`
  (params (ActionValue :type Boolean) (ElapsedSeconds :type "Float (double-precision)") (TriggeredSeconds :type "Float (double-precision)") (InputAction :type "InputAction Object Reference" :default "/Game/Game/Input/Dash.Dash"))
  (bind _voiture_ (`self.Voiture_`))
  ;[0.6533 0.6691 1] Dash
  (:`Triggered`
    (`|ExecutionSequence`
      (:`then_0`
        (`/Engine/EditorBlueprintResources/StandardMacros.Gate` false :!label _label_4
          (:`Exit`
            (`PrimitiveComponent.AddImpulse` _voiture_ (* (`SceneComponent.GetForwardVector` _voiture_) (`self.Puissance Dash`)) "None" true)
            ;[0.3812 0.6277 1] Passage à travers le mur
            (bind _outactors (`GameplayStatics.GetAllActorsOfClass` "/Game/Level_Design/MecaniquesLD/BP_DashWall.BP_DashWall_C"))
            (`/Game/Level_Design/MecaniquesLD/BP_DashWall.DashSetCollision` _outactors)
            (`PrimitiveComponent.SetMaterial` (`self.Voiture_`) 0 "/Game/Maletial/M_DashEffect.M_DashEffect")
            (`PrimitiveComponent.SetMaterial` (`self.Skin_Liam`) 0 "/Game/Maletial/M_DashEffect.M_DashEffect")
            (`KismetSystemLibrary.Delay` 0.2) ; Dois être égale à "Temps effet dash" dans le BP_DashWall
            (`PrimitiveComponent.SetMaterial` (`self.Voiture_`) 0 "/Engine/BasicShapes/BasicShapeMaterial.BasicShapeMaterial")
            (`PrimitiveComponent.SetMaterial` (`self.Skin_Liam`) 0 "/Engine/BasicShapes/BasicShapeMaterial.BasicShapeMaterial"))))
      (:`then_1`
        (`KismetSystemLibrary.Delay` (`self.Cooldown Dash (sec)`))
        (goto _label_4 :!via `Open`))
      (:`then_2`
        (goto _label_4 :!via `Close`)))))

(fn `UserConstructionScript`)