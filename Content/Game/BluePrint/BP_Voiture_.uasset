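; Player-possessed, physics-driven car that drives through forces and torque, counts checkpoint laps and notifies spawners on each lap.
; A downward trace each Tick sets air/ground damping, aligns the visible mesh to slopes and controls a timeline fall force.
; Input adds a cooldown dash through BP_DashWall, an expanding horn sphere, headlights, six-skin cycling and a menu toggle.
; Overlapping the Moisson actor or pressing restart opens Level_Chambre.
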(event `self.ReceiveBeginPlay`
  (bind _returnvalue (pcsubsystem `EnhancedInputLocalPlayerSubsystem` (`GameplayStatics.GetPlayerController` 0)))
  (`Controller.Possess` (`GameplayStatics.GetPlayerController` 0) self)
  (bind _output_get (set `self.Selected_VoitureRef` (`self.WSV_Asset_Voiture_liam`)))
  (`SceneComponent.SetHiddenInGame` _output_get false false)
  (`|ExecutionSequence`
    (:`then_0`
      ;[0.2379 0.7249 1] Set Up Index BP_SpawnTours
      (for _array_element (`self.ActorsWithSpawnTours`)
        (for _array_element_2 (`self.GetComponentsByInterface` _array_element "/Game/Game/BluePrint/BPI_Distribute.BPI_Distribute_C")
          (`KismetArrayLibrary.Array_Add` (`self.BP_SpawnTours`) _array_element_2))))
    (:`then_1`
      (bind _outactors (`GameplayStatics.GetAllActorsOfClass` "/Game/Level_Design/MecaniquesLD/BP_CheckPoint.BP_CheckPoint_C"))
      (set `self.NbCheckPoint` (`KismetArrayLibrary.Array_Length` _outactors))
      (`PrimitiveComponent.SetLinearDamping` (`self.Voiture_`) (`self.Linear Damping`))
      (`PrimitiveComponent.SetAngularDamping` (`self.Voiture_`) (`self.Angular Damping`))
      (bind _outactors_2 (`GameplayStatics.GetAllActorsWithInterface` "/Game/Game/BluePrint/BPI_Distribute.BPI_Distribute_C"))
      (for _array_element_3 _outactors_2
        (`KismetArrayLibrary.Array_Add` (`self.BPI_Distribute_Actors`) _array_element_3)
        (message `/Game/Game/BluePrint/BPI_Distribute.Distriubte_VoitureVariable` (`self.BPI_Distribute_Actors`) self))
      ;[0 1 0.06418] Input Local Player
      (`/Engine/EditorBlueprintResources/StandardMacros.IsValid` _returnvalue
        (:`Is Valid`
          (`EnhancedInputSubsystemInterface.AddMappingContext` _returnvalue "/Game/Game/Input/IM_Voiture.IM_Voiture" 0 (struct)))))))

(event `/Game/Game/BluePrint/BPI_Distribute.Distribute_ActorsWithSpawnTours`
  (params (Actors :type "Actor Object Reference"))
  (`KismetArrayLibrary.Array_Add` (`self.ActorsWithSpawnTours`) Actors))

(event `EnhancedInput|/Game/Game/Input/IA_SwapVoiture`
  (params (ActionValue :type Boolean) (ElapsedSeconds :type "Float (double-precision)") (TriggeredSeconds :type "Float (double-precision)") (InputAction :type "InputAction Object Reference" :default "/Game/Game/Input/IA_SwapVoiture.IA_SwapVoiture"))
  ;[1 1 1] SwapVoiture
  (:`Started`
    (`|MultiGate` false true
      (:`Out 0`
        (set `self.Selected_VoitureRef` (`self.SM_voiturePierre`))
        (`SceneComponent.SetHiddenInGame` (`self.WSV_Asset_Voiture_liam`) true false)
        (`SceneComponent.SetHiddenInGame` (`self.WSV_Asset_Voiture_Champi_02`) true false)
        (`SceneComponent.SetHiddenInGame` (`self.SM_VoitureJulienVerte`) true false)
        (`SceneComponent.SetHiddenInGame` (`self.SM_voitureEmma`) true false)
        (`SceneComponent.SetHiddenInGame` (`self.WSV_Asset_VoitureVamp`) true false))
      (:`Out 1`
        (set `self.Selected_VoitureRef` (`self.WSV_Asset_VoitureVamp`))
        (`SceneComponent.SetHiddenInGame` (`self.WSV_Asset_Voiture_liam`) true false)
        (`SceneComponent.SetHiddenInGame` (`self.SM_voiturePierre`) true false)
        (`SceneComponent.SetHiddenInGame` (`self.SM_voitureEmma`) true false)
        (`SceneComponent.SetHiddenInGame` (`self.SM_VoitureJulienVerte`) true false)
        (`SceneComponent.SetHiddenInGame` (`self.WSV_Asset_Voiture_Champi_02`) true false))
      (:`Out 2`
        (set `self.Selected_VoitureRef` (`self.WSV_Asset_Voiture_liam`))
        (`SceneComponent.SetHiddenInGame` (`self.WSV_Asset_Voiture_Champi_02`) true false)
        (`SceneComponent.SetHiddenInGame` (`self.SM_VoitureJulienVerte`) true false)
        (`SceneComponent.SetHiddenInGame` (`self.SM_voitureEmma`) true false)
        (`SceneComponent.SetHiddenInGame` (`self.WSV_Asset_VoitureVamp`) true false)
        (`SceneComponent.SetHiddenInGame` (`self.SM_voiturePierre`) true false))
      (:`Out 3`
        (set `self.Selected_VoitureRef` (`self.WSV_Asset_Voiture_Champi_02`))
        (`SceneComponent.SetHiddenInGame` (`self.WSV_Asset_Voiture_liam`) true false)
        (`SceneComponent.SetHiddenInGame` (`self.SM_VoitureJulienVerte`) true false)
        (`SceneComponent.SetHiddenInGame` (`self.SM_voitureEmma`) true false)
        (`SceneComponent.SetHiddenInGame` (`self.WSV_Asset_VoitureVamp`) true false)
        (`SceneComponent.SetHiddenInGame` (`self.SM_voiturePierre`) true false))
      (:`Out 4`
        (set `self.Selected_VoitureRef` (`self.SM_VoitureJulienVerte`))
        (`SceneComponent.SetHiddenInGame` (`self.WSV_Asset_Voiture_liam`) true false)
        (`SceneComponent.SetHiddenInGame` (`self.WSV_Asset_Voiture_Champi_02`) true false)
        (`SceneComponent.SetHiddenInGame` (`self.SM_voitureEmma`) true false)
        (`SceneComponent.SetHiddenInGame` (`self.WSV_Asset_VoitureVamp`) true false)
        (`SceneComponent.SetHiddenInGame` (`self.SM_voiturePierre`) true false))
      (:`Out 5`
        (set `self.Selected_VoitureRef` (`self.SM_voitureEmma`))
        (`SceneComponent.SetHiddenInGame` (`self.WSV_Asset_Voiture_liam`) true false)
        (`SceneComponent.SetHiddenInGame` (`self.WSV_Asset_Voiture_Champi_02`) true false)
        (`SceneComponent.SetHiddenInGame` (`self.SM_VoitureJulienVerte`) true false)
        (`SceneComponent.SetHiddenInGame` (`self.WSV_Asset_VoitureVamp`) true false)
        (`SceneComponent.SetHiddenInGame` (`self.SM_voiturePierre`) true false)))
    (`KismetSystemLibrary.PrintString` "Hello" false)
    (`SceneComponent.SetHiddenInGame` (`self.Selected_VoitureRef`) false false)))

(event `/Game/Game/BluePrint/BPI_Distribute.Tours`
  (bind _bp_spawntours (`self.BP_SpawnTours`))
  ;[0.328 1 0.07785] Tours
  (if (>= (`self.CheckPointValide`) (`self.NbCheckPoint`))
    (`/Engine/EditorBlueprintResources/StandardMacros.IncrementInt` (`self.Tours_`)
      (:`  `
        (set `self.CheckPointValide` 0)
        (`KismetSystemLibrary.PrintString` (`KismetStringLibrary.Conv_IntToString` (`self.Tours_`)) false false (struct :`R` 1.0 :`G` 0.110987 :`A` 1.0))
        (bind _outactors (`GameplayStatics.GetAllActorsOfClass` "/Game/Level_Design/MecaniquesLD/BP_CheckPoint.BP_CheckPoint_C"))
        (`/Game/Level_Design/MecaniquesLD/BP_CheckPoint.LapDone_CusEvnt` _outactors)
        (`KismetSystemLibrary.PrintString` "LapDone" false)
        (for _array_element _bp_spawntours
          (`/Engine/EditorBlueprintResources/StandardMacros.IsValid` _array_element
            (:`Is Valid`
              (message `/Game/Game/BluePrint/BPI_Distribute.+1Tours` _array_element))
            (:`Is Not Valid`
              (`KismetArrayLibrary.Array_RemoveItem` _bp_spawntours _array_element))))))))

(event `EnhancedInput|/Game/Game/Input/Phare`
  (params (ActionValue :type Boolean) (ElapsedSeconds :type "Float (double-precision)") (TriggeredSeconds :type "Float (double-precision)") (InputAction :type "InputAction Object Reference" :default "/Game/Game/Input/Phare.Phare"))
  ;[0.3333 0.6781 1] Phares on/off
  (:`Started`
    (`SceneComponent.ToggleVisibility` (`self.PharesL`) false)
    (`SceneComponent.ToggleVisibility` (`self.PharesR`) false)))

(event `Key|AnyKey`
  (params (Key :type "Key Structure"))
  ;[1 0.9727 0.1531] DebugKey
)

(event `/Game/Game/BluePrint/BPI_Distribute.CheckPoint Valide`
  ;[0 0.1335 1] CheckPoint
  (bind _result (`/Engine/EditorBlueprintResources/StandardMacros.IncrementInt` (`self.CheckPointValide`))
    (:`  `
      (`KismetSystemLibrary.PrintString` (`KismetStringLibrary.Conv_IntToString` _result) false false (struct :`G` 0.118933 :`B` 1.0 :`A` 1.0)))))

(event `EnhancedInput|/Game/Game/Input/Forward_Backward`
  (params (ActionValue :type "Float (double-precision)") (ElapsedSeconds :type "Float (double-precision)") (TriggeredSeconds :type "Float (double-precision)") (InputAction :type "InputAction Object Reference" :default "/Game/Game/Input/Forward_Backward.Forward_Backward"))
  ;[0.133 0.2084 1] Movement Z_S
  (:`Triggered`
    (set `self.Backward` (== -1.0 ActionValue))
    (if (`self.In air`)
      _
      (elif (`self.Backward`)
        (`self.AddForce` -1.0 (`self.VitesseBackward`))
        (else
          (`self.AddForce` 1.0 (`self.Vitesse Voiture`))))))
  (:`Completed`
    (set `self.Backward` false)))

(event `EnhancedInput|/Game/Game/Input/IA_UI`
  (params (ActionValue :type Boolean) (ElapsedSeconds :type "Float (double-precision)") (TriggeredSeconds :type "Float (double-precision)") (InputAction :type "InputAction Object Reference" :default "/Game/Game/Input/IA_UI.IA_UI"))
  ;[1 1 1] UI
  (:`Started`
    (`/Engine/EditorBlueprintResources/StandardMacros.FlipFlop`
      (:`A`
        (bind _returnvalue (`|CreateWidget` "/Game/Game/Menu/WBP_Menu.WBP_Menu_C"))
        (`UserWidget.AddToViewport` _returnvalue 0)
        (set `PlayerController.bShowMouseCursor` true (`GameplayStatics.GetPlayerController` 0)))
      (:`B`
        (`WidgetLayoutLibrary.RemoveAllWidgets`)))))

(event `/Game/Game/BluePrint/BPI_Distribute.Distribute_MoissonVariable`
  (params (MoissonReference :type "/Game/Game/BluePrint/BP_LaMoisson Object Reference"))
  (set `self.Moisson Reference` MoissonReference))

(event `self.Voiture_.OnComponentBeginOverlap`
  (params (OverlappedComponent :type "PrimitiveComponent Object Reference") (OtherActor :type "Actor Object Reference") (OtherComp :type "PrimitiveComponent Object Reference") (OtherBodyIndex :type Integer) (bFromSweep :type Boolean) (SweepResult :type "HitResult Structure (by ref)"))
  ;[0.7338 0.8643 1] Slow when overlap RedCube *(aka : killercube)
  (if (== OtherActor (`self.Moisson Reference`))
    ;[0.757 1 0.7609] Restart when press R
    (`GameplayStatics.OpenLevelBySoftObjectPtr` "/Game/Level/Level_Chambre.Level_Chambre" :!label _label)))

(event `RedCube_SlowOverlap`
  ;[0.7338 0.8643 1] Slow when overlap RedCube *(aka : killercube)
  (bind _result (`/Engine/EditorBlueprintResources/StandardMacros.NegateFloat` (`self.SlowCube_ForceEffect`))
    (:`  `
      (`KismetSystemLibrary.PrintString` "Hello" false))))

(event `EnhancedInput|/Game/Game/Input/Left_Right`
  (params (ActionValue :type "Float (double-precision)") (ElapsedSeconds :type "Float (double-precision)") (TriggeredSeconds :type "Float (double-precision)") (InputAction :type "InputAction Object Reference" :default "/Game/Game/Input/Left_Right.Left_Right"))
  (bind _torquemax (`self.TorqueMax`))
  ;[0.07881 0.1091 0.4072] Movement Q_D
  (:`Triggered`
    (if (`self.In air`)
      (bind (_direction _courbe) (`Timeline|CourbeVirage` :!via `Reverse` :!label _label_2)
        (:`Update`
          (if (`self.Backward`)
            (bind _result (`/Engine/EditorBlueprintResources/StandardMacros.NegateFloat` ActionValue)
              (:`  `
                (`self.AddForceInDegrees` _courbe _result _torquemax)))
            (else
              (`self.AddForceInDegrees` _courbe ActionValue _torquemax)))))
      (else
        (goto _label_2))))
  (:`Completed`
    (`|ExecutionSequence`
      (:`then_0`
        (goto _label_2 :!via `Stop`))
      (:`then_1`
        (goto _label_2 :!via `SetNewTime`)))))

(event `EnhancedInput|/Game/Game/Input/Klaxon`
  (params (ActionValue :type Boolean) (ElapsedSeconds :type "Float (double-precision)") (TriggeredSeconds :type "Float (double-precision)") (InputAction :type "InputAction Object Reference" :default "/Game/Game/Input/Klaxon.Klaxon"))
  ;[1 0.8746 0.8845] Wave
  (:`Triggered`
    (bind (_direction _wave) (`Timeline|Wave` :!via `PlayFromStart`)
      (:`Update`
        (`SphereComponent.SetSphereRadius` (`self.Klaxon`) (* _wave (`self.WaveRadius`)) true))
      (:`Finished`
        (`SphereComponent.SetSphereRadius` (`self.Klaxon`) 0.0 true)))))

(event `EnhancedInput|/Game/Game/Input/IA_Restart`
  (params (ActionValue :type Boolean) (ElapsedSeconds :type "Float (double-precision)") (TriggeredSeconds :type "Float (double-precision)") (InputAction :type "InputAction Object Reference" :default "/Game/Game/Input/IA_Restart.IA_Restart"))
  ;[0.757 1 0.7609] Restart when press R
  (:`Started`
    (goto _label)))

(event `self.ReceiveTick`
  (params (DeltaSeconds :type "Float (single-precision)"))
  (bind _selected_voitureref (`self.Selected_VoitureRef`))
  (bind _returnvalue (`SceneComponent.K2_GetComponentLocation` (`self.Voiture_`)))
  ;[0.204 0.3748 1] Movement air_control
  (`|ExecutionSequence`
    (:`then_0`
      (bind (_outhit _returnvalue_2) (`KismetSystemLibrary.LineTraceSingle` _returnvalue (+ _returnvalue (* (`SceneComponent.GetUpVector` (`self.Voiture_`)) -200.0)) "TraceTypeQuery1"))
      (if _returnvalue_2
        (`|ExecutionSequence`
          (:`then_0`
            (`self.SetLinearDamping_Air` (`self.Linear Damping`))
            (bind (_direction _courberetomber) (`Timeline|CourbeRetomber` :!via `Stop` :!label _label_3)
              (:`Update`
                (bind _result (`/Engine/EditorBlueprintResources/StandardMacros.NegateFloat` (* _courberetomber (`self.ForceDeRetomber`)))
                  (:`  `
                    (`PrimitiveComponent.AddForce` (`self.Voiture_`) (`KismetMathLibrary.MakeVector` 0.0 0.0 _result) "None" true))))))
          (:`then_1`
            ;[0.6676 0.8217 1] Ouais Ouais
            (`SceneComponent.K2_SetWorldRotation` _selected_voitureref (`KismetMathLibrary.RInterpTo` (`SceneComponent.K2_GetComponentRotation` _selected_voitureref) (`KismetMathLibrary.MakeRotator` (* (- (.pitch (`KismetMathLibrary.Conv_VectorToRotator` (`.Normal` (`GameplayStatics.BreakHitResult` _outhit)))) 90.0) -1.0) (.roll (`KismetMathLibrary.Conv_VectorToRotator` (`.Normal` (`GameplayStatics.BreakHitResult` _outhit)))) (.yaw (`SceneComponent.K2_GetComponentRotation` (`self.Selected_VoitureRef`)))) (`GameplayStatics.GetWorldDeltaSeconds`) 20.0) false true)))
        (else
          (`self.SetLinearDamping_Air` (`self.Linear damping in air`) true)
          (goto _label_3 :!via `PlayFromStart`))))))

(event `EnhancedInput|/Game/Game/Input/Dash`
  (params (ActionValue :type Boolean) (ElapsedSeconds :type "Float (double-precision)") (TriggeredSeconds :type "Float (double-precision)") (InputAction :type "InputAction Object Reference" :default "/Game/Game/Input/Dash.Dash"))
  (bind _voiture_ (`self.Voiture_`))
  ;[0.6533 0.6691 1] Dash
  (:`Triggered`
    (if (not (`self.In air`))
      (`|ExecutionSequence`
        (:`then_0`
          (`/Engine/EditorBlueprintResources/StandardMacros.Gate` false :!label _label_4
            (:`Exit`
              (`PrimitiveComponent.AddImpulse` _voiture_ (* (`SceneComponent.GetForwardVector` _voiture_) (`self.Puissance Dash`)) "None" true)
              ;[0.3812 0.6277 1] Passage à travers le mur
              (bind _outactors (`GameplayStatics.GetAllActorsOfClass` "/Game/Level_Design/MecaniquesLD/BP_DashWall.BP_DashWall_C"))
              (`/Game/Level_Design/MecaniquesLD/BP_DashWall.DashSetCollision` _outactors)
              (`PrimitiveComponent.SetMaterial` (`self.Voiture_`) 0 "/Game/Asset_3D/Maletial/Material_GD/M_DashEffect.M_DashEffect")
              (`KismetSystemLibrary.Delay` 0.4) ; Dois être égale à "Temps effet dash" dans le BP_DashWall
              (`PrimitiveComponent.SetMaterial` (`self.Voiture_`) 0 "/Engine/BasicShapes/BasicShapeMaterial.BasicShapeMaterial"))))
        (:`then_1`
          (`KismetSystemLibrary.Delay` (`self.Cooldown Dash (sec)`))
          (goto _label_4 :!via `Open`))
        (:`then_2`
          (goto _label_4 :!via `Close`))))))

(fn `AddForce`
  (params (InputValue :type "Float (double-precision)") (Vitesse :type "Float (double-precision)"))
  (`PrimitiveComponent.AddForce` (`self.Voiture_`) (* (* Vitesse InputValue) (`SceneComponent.GetForwardVector` (`self.Voiture_`))) "None" true))

(fn `AddForceInDegrees`
  (params (Courbe :type "Float (double-precision)") (ActionValue :type "Float (double-precision)") (TorqueMax :type "Float (double-precision)"))
  (`PrimitiveComponent.AddTorqueInDegrees` (`self.Voiture_`) (`KismetMathLibrary.MakeVector` 0.0 0.0 (* (* TorqueMax Courbe) ActionValue)) "None" true))

(fn `Distriubte_VoitureVariable`
  (params (BP_Voiture :type "/Game/Game/BluePrint/BP_Voiture_ Object Reference")))

(fn `SetLinearDamping_Air`
  (params (InDamping :type "Float (single-precision)") (`In air` :type Boolean))
  (set `self.In air` `In air`)
  (`PrimitiveComponent.SetLinearDamping` (`self.Voiture_`) InDamping))

(fn `UserConstructionScript`)