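; Boost pad for level design that launches the car forward when it drives over it.
; When a component tagged "Voiture" enters the box, it finds the car with GetActorOfClass rather than using the overlapping actor.
; It applies a velocity-change impulse along the car's own forward vector, ignoring pad orientation.
; The plate then briefly swaps to a "used" material before reverting after a short delay.
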(event `self.Box.OnComponentBeginOverlap`
  (params (OverlappedComponent :type "PrimitiveComponent Object Reference") (OtherActor :type "Actor Object Reference") (OtherComp :type "PrimitiveComponent Object Reference") (OtherBodyIndex :type Integer) (bFromSweep :type Boolean) (SweepResult :type "HitResult Structure (by ref)"))
  (if (`ActorComponent.ComponentHasTag` OtherComp "Voiture")
    (bind _returnvalue (`GameplayStatics.GetActorOfClass` "/Game/Game/BluePrint/BP_Voiture.BP_Voiture_C"))
    (bind _voiture (`/Game/Game/BluePrint/BP_Voiture.Voiture` _returnvalue))
    (`PrimitiveComponent.AddImpulse` _voiture (* 6000.0 (`SceneComponent.GetForwardVector` _voiture)) "None" true)
    (`PrimitiveComponent.SetMaterial` (`self.Plaque`) 0 "/Game/Maletial/M_PadUse.M_PadUse")
    (`KismetSystemLibrary.Delay` 0.1)
    (`PrimitiveComponent.SetMaterial` (`self.Plaque`) 0 "/Game/Maletial/M_BoostPad.M_BoostPad")))

(fn `UserConstructionScript`)