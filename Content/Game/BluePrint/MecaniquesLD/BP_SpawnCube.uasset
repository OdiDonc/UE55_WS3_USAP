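; BP_SpawnCube is a spawner that keeps creating BP_Walker actors around its Box component, with no count limit.
; Tick feeds a 0.3-second Delay, which paces the spawns.
; Each spawn location adds random per-axis offsets, derived from the box's scaled extent, to the box's world location.
; The Z offset range uses zero divided by the extent as its minimum, unlike X and Y, which use half the extent.
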(event `self.ReceiveTick`
  (params (DeltaSeconds :type "Float (single-precision)"))
  (bind (_returnvalue_x _returnvalue_y _returnvalue_z) (`KismetMathLibrary.BreakVector` (`BoxComponent.GetScaledBoxExtent` (`self.Box`))))
  (bind (_returnvalue_x_2 _returnvalue_y_2 _returnvalue_z_2) (`KismetMathLibrary.BreakVector` (`SceneComponent.K2_GetComponentLocation` (`self.Box`))))
  (`KismetSystemLibrary.Delay` 0.3)
  (bind _result (`/Engine/EditorBlueprintResources/StandardMacros.NegateFloat` _returnvalue_x)
    (:`  `
      (bind _result_2 (`/Engine/EditorBlueprintResources/StandardMacros.NegateFloat` _returnvalue_y)
        (:`  `
          (bind _result_3 (`/Engine/EditorBlueprintResources/StandardMacros.NegateFloat` _returnvalue_z)
            (:`  `
              (`|SpawnActorFromClass` "/Game/Game/BluePrint/MecaniquesLD/BP_Walker.BP_Walker_C" (`KismetMathLibrary.MakeTransform` (`KismetMathLibrary.MakeVector` (+ _returnvalue_x_2 (`KismetMathLibrary.RandomFloatInRange` (/ _returnvalue_x 2.0) _result)) (+ _returnvalue_y_2 (`KismetMathLibrary.RandomFloatInRange` (/ _returnvalue_y 2.0) _result_2)) (+ _returnvalue_z_2 (`KismetMathLibrary.RandomFloatInRange` (/ 0.0 _returnvalue_z) _result_3)))) "Undefined" "MultiplyWithRoot" null null))))))))

(fn `UserConstructionScript`)