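; BP_Walker is a level-design mechanic: a physics cube that the car's horn knocks away and freeze volumes lock in place.
; Overlapping a "Klaxon"-tagged component traces from BP_Voiture to the cube and applies an impulse opposite the hit normal, with added lift.
; Overlapping a "Freez"-tagged component disables physics and closes the gate on that impulse; leaving it restores both.
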(event `self.Walker_Cube.OnComponentBeginOverlap`
  (params (OverlappedComponent :type "PrimitiveComponent Object Reference") (OtherActor :type "Actor Object Reference") (OtherComp :type "PrimitiveComponent Object Reference") (OtherBodyIndex :type Integer) (bFromSweep :type Boolean) (SweepResult :type "HitResult Structure (by ref)"))
  (`|ExecutionSequence`
    (:`then_0`
      ;[0 0.9629 1] FeedBack_Klaxon
      (if (`ActorComponent.ComponentHasTag` OtherComp "Klaxon")
        (bind _returnvalue (`GameplayStatics.GetActorOfClass` "/Game/Game/BluePrint/BP_Voiture.BP_Voiture_C"))
        (bind _outhit (`KismetSystemLibrary.LineTraceSingle` (`SceneComponent.K2_GetComponentLocation` (`/Game/Game/BluePrint/BP_Voiture.Voiture` _returnvalue)) (`SceneComponent.K2_GetComponentLocation` (`self.Walker_Cube`)) "TraceTypeQuery1"))
        (`/Engine/EditorBlueprintResources/StandardMacros.Gate` false :!label _label
          (:`Exit`
            (`PrimitiveComponent.SetSimulatePhysics` (`self.Walker_Cube`) true)
            (`PrimitiveComponent.AddImpulse` (`self.Walker_Cube`) (+ (* (`.ImpactNormal` (`GameplayStatics.BreakHitResult` _outhit)) -2000.0) (0.0 0.0 600.0)) "None" true)))))
    (:`then_1`
      ;[0.1015 0 1] Freez
      (if (`ActorComponent.ComponentHasTag` OtherComp "Freez")
        (`PrimitiveComponent.SetSimulatePhysics` (`self.Walker_Cube`) false)
        (goto _label :!via `Close`)))))

(event `self.Walker_Cube.OnComponentEndOverlap`
  (params (OverlappedComponent :type "PrimitiveComponent Object Reference") (OtherActor :type "Actor Object Reference") (OtherComp :type "PrimitiveComponent Object Reference") (OtherBodyIndex :type Integer))
  ;[0.1015 0 1] Freez
  (if (`ActorComponent.ComponentHasTag` OtherComp "Freez")
    (`PrimitiveComponent.SetSimulatePhysics` (`self.Walker_Cube`) true)
    (goto _label :!via `Open`)))

(fn `UserConstructionScript`)