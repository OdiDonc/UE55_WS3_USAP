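; Walker actor, a cube that gets knocked away when it overlaps the horn (Klaxon) of BP_Voiture.
; On overlap with a Klaxon-tagged component, it traces from the car to itself, enables physics and applies an impulse against the hit normal plus an upward lift.
; A gated headlight freeze check (FreezPhares, Freez tag) only prints debug text, and the physics-toggling freeze logic is disconnected.
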(event `self.Walker_Cube.OnComponentBeginOverlap`
  (params (OverlappedComponent :type "PrimitiveComponent Object Reference") (OtherActor :type "Actor Object Reference") (OtherComp :type "PrimitiveComponent Object Reference") (OtherBodyIndex :type Integer) (bFromSweep :type Boolean) (SweepResult :type "HitResult Structure (by ref)"))
  (bind _walker_cube (`self.Walker_Cube`))
  (`|ExecutionSequence`
    (:`then_0`
      ;[0.8547 1 0] FeedBack_Klaxon
      (if (`ActorComponent.ComponentHasTag` OtherComp "Klaxon")
        (bind _returnvalue (`GameplayStatics.GetActorOfClass` "/Game/Game/BluePrint/BP_Voiture.BP_Voiture_C"))
        (bind _outhit (`KismetSystemLibrary.LineTraceSingle` (`SceneComponent.K2_GetComponentLocation` (`/Game/Game/BluePrint/BP_Voiture.Voiture` _returnvalue)) (`SceneComponent.K2_GetComponentLocation` (`self.Walker_Cube`)) "TraceTypeQuery1"))
        (`PrimitiveComponent.SetSimulatePhysics` _walker_cube true)
        (`PrimitiveComponent.AddImpulse` _walker_cube (+ (* (`.ImpactNormal` (`GameplayStatics.BreakHitResult` _outhit)) -2000.0) (0.0 0.0 600.0)) "None" true)
        (if (`SceneComponent.IsSimulatingPhysics` (`self.Walker_Cube`) "None")
          (if false
            (`KismetSystemLibrary.PrintString` "True" true true (struct :`R` 0.247905 :`G` 0.25828 :`B` 1.0 :`A` 1.0))
            (`KismetSystemLibrary.PrintString` "Github" true true (struct :`A` 1.0))
            (else
              (`KismetSystemLibrary.PrintString` "False" true true (struct :`R` 0.322917 :`G` 0.6557 :`B` 1.0 :`A` 1.0)))))))
    (:`then_1`
      ;[1 1 1] Freez
      (`/Engine/EditorBlueprintResources/StandardMacros.Gate` true
        (:`Exit`
          (bind _asbp_voiture (cast `/Game/Game/BluePrint/BP_Voiture` OtherActor))
          (if (`ActorComponent.ComponentHasTag` (`/Game/Game/BluePrint/BP_Voiture.FreezPhares` _asbp_voiture) "Freez")
            (`KismetSystemLibrary.PrintString` "True" true true (struct :`R` 1.0 :`G` 0.037924 :`A` 1.0))
            (else
              (`KismetSystemLibrary.PrintString` "False" true true (struct :`R` 1.0 :`G` 0.037924 :`A` 1.0)))))))))

(event `self.Walker_Cube.OnComponentEndOverlap`
  (params (OverlappedComponent :type "PrimitiveComponent Object Reference") (OtherActor :type "Actor Object Reference") (OtherComp :type "PrimitiveComponent Object Reference") (OtherBodyIndex :type Integer))
  ;[1 1 1] Freez
  (if true
    _))

(fn `UserConstructionScript`)