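; BP_BoostPad is a level-design boost pad that propels the car forward when a component tagged "Voiture" enters its box.
; It fetches BP_Voiture through GetActorOfClass rather than the overlapping actor, then applies a mass-independent velocity-change impulse along the car's forward vector, scaled by PuissanceBoost.
; The plate briefly swaps to a used material as feedback, and the pad can optionally destroy itself after a configurable delay.
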(event `self.Box.OnComponentBeginOverlap`
  (params (OverlappedComponent :type "PrimitiveComponent Object Reference") (OtherActor :type "Actor Object Reference") (OtherComp :type "PrimitiveComponent Object Reference") (OtherBodyIndex :type Integer) (bFromSweep :type Boolean) (SweepResult :type "HitResult Structure (by ref)"))
  (if (`ActorComponent.ComponentHasTag` OtherComp "Voiture")
    (bind _returnvalue (`GameplayStatics.GetActorOfClass` "/Game/Game/BluePrint/BP_Voiture.BP_Voiture_C"))
    (bind _voiture_ (`/Game/Game/BluePrint/BP_Voiture.Voiture_` _returnvalue))
    (`PrimitiveComponent.AddImpulse` _voiture_ (* (`self.PuissanceBoost`) (`SceneComponent.GetForwardVector` _voiture_)) "None" true)
    (`PrimitiveComponent.SetMaterial` (`self.Plaque`) 0 "/Game/Asset_3D/Maletial/Material_GD/M_PadUse.M_PadUse")
    (`KismetSystemLibrary.Delay` 0.1)
    (`PrimitiveComponent.SetMaterial` (`self.Plaque`) 0 "/Game/Asset_3D/Maletial/Material_GD/M_BoostPad.M_BoostPad")
    (if (`self.MortApresUtilisation?`)
      (`KismetSystemLibrary.Delay` (`self.MortApresUtilisation(Sec)`))
      (`self.K2_DestroyActor`))))

(fn `UserConstructionScript`)