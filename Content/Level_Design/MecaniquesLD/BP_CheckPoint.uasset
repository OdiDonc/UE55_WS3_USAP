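; BP_CheckPoint is a race checkpoint that reports when a BP_Voiture car passes through its trigger box.
; On BeginPlay it scans actors implementing BPI_Distribute and keeps the last one found.
; An overlap by the car's Voiture component sends that actor CheckPointValideMessage through a DoOnce gate, so it counts once until LapDone_CusEvnt resets the gate.
; The Tours function is an empty stub.
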(event `self.ReceiveBeginPlay`
  (bind _outactors (`GameplayStatics.GetAllActorsWithInterface` "/Game/Game/BluePrint/BPI_Distribute.BPI_Distribute_C"))
  (for _array_element _outactors
    (set `self.BPI_Distribute_Actors` _array_element)))

(event `self.Box.OnComponentBeginOverlap`
  (params (OverlappedComponent :type "PrimitiveComponent Object Reference") (OtherActor :type "Actor Object Reference") (OtherComp :type "PrimitiveComponent Object Reference") (OtherBodyIndex :type Integer) (bFromSweep :type Boolean) (SweepResult :type "HitResult Structure (by ref)"))
  (bind _asbp_voiture (cast `/Game/Game/BluePrint/BP_Voiture` OtherActor))
  (if (== (`/Game/Game/BluePrint/BP_Voiture.Voiture_` _asbp_voiture) OtherComp)
    (`/Engine/EditorBlueprintResources/StandardMacros.DoOnce` false :!label _label
      (:`Completed`
        (message `/Game/Game/BluePrint/BPI_Distribute.CheckPoint Valide` (`self.BPI_Distribute_Actors`))))))

(event `LapDone_CusEvnt`
  (goto _label :!via `Reset`))

(fn `Tours`
  (return))

(fn `UserConstructionScript`)