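; BP_CubeKiller is a level-design cube obstacle that slows the player's car on contact and can be knocked away with the horn.
; Its overlap event calls the car's RedCubeSlowOverlap for the body, while the Klaxon component enables physics and launches the cube.
; The impulse combines a car-to-cube trace's impact normal with vertical lift, optionally followed by delayed destruction.
; The car reference arrives through DistriubteVoitureVariable.
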(event `self.Walker_Cube.OnComponentBeginOverlap`
  (params (OverlappedComponent :type "PrimitiveComponent Object Reference") (OtherActor :type "Actor Object Reference") (OtherComp :type "PrimitiveComponent Object Reference") (OtherBodyIndex :type Integer) (bFromSweep :type Boolean) (SweepResult :type "HitResult Structure (by ref)"))
  (bind _bp_voiture (`self.BP Voiture`))
  ;[0 0.9629 1] FeedBack_Klaxon
  (`/Engine/EditorBlueprintResources/StandardMacros.IsValid` _bp_voiture
    (:`Is Valid`
      (`|ExecutionSequence`
        (:`then_0`
          (if (== OtherComp (`/Game/Game/BluePrint/BP_Voiture.Voiture_` _bp_voiture))
            (`/Game/Game/BluePrint/BP_Voiture.RedCube_SlowOverlap` _bp_voiture)))
        (:`then_1`
          (if (== OtherComp (`/Game/Game/BluePrint/BP_Voiture.Klaxon` _bp_voiture))
            (bind _outhit (`KismetSystemLibrary.LineTraceSingle` (`SceneComponent.K2_GetComponentLocation` (`/Game/Game/BluePrint/BP_Voiture.Voiture_` _bp_voiture)) (`SceneComponent.K2_GetComponentLocation` (`self.Walker_Cube`)) "TraceTypeQuery1"))
            (`PrimitiveComponent.SetSimulatePhysics` (`self.Walker_Cube`) true)
            (`PrimitiveComponent.AddImpulse` (`self.Walker_Cube`) (+ (* (`.ImpactNormal` (`GameplayStatics.BreakHitResult` _outhit)) (`self.Puissance Klaxon X;Y`)) (`KismetMathLibrary.MakeVector` 0.0 0.0 (`self.Puissance Klaxon Z`))) "None" true)
            (if (`self.MortApresKlaxon?`)
              (`KismetSystemLibrary.Delay` (`self.MortApresKlaxon(Sec)`))
              (`self.K2_DestroyActor`))))))))

(event `/Game/Game/BluePrint/BPI_Distribute.Distriubte_VoitureVariable`
  (params (BP_Voiture :type "/Game/Game/BluePrint/BP_Voiture Object Reference"))
  (set `self.BP Voiture` BP_Voiture))

(fn `UserConstructionScript`)