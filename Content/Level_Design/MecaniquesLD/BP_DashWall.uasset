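; BP_DashWall is a level-design wall that temporarily lets objects pass through as the effect of a dash.
; The DashSetCollision event sets the wall to overlap all channels, waits for a configurable effect duration, then restores full blocking.
; When a component tagged "Voiture" (car) begins overlapping, the wall briefly swaps to an overlap material as feedback, then switches to the dash-effect material.
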(event `self.DashWall.OnComponentBeginOverlap`
  (params (OverlappedComponent :type "PrimitiveComponent Object Reference") (OtherActor :type "Actor Object Reference") (OtherComp :type "PrimitiveComponent Object Reference") (OtherBodyIndex :type Integer) (bFromSweep :type Boolean) (SweepResult :type "HitResult Structure (by ref)"))
  (if (`ActorComponent.ComponentHasTag` OtherComp "Voiture")
    ;[0.256 0.4491 1] FeedBack - Wall Overlap
    (`PrimitiveComponent.SetMaterial` (`self.DashWall`) 0 "/Game/Asset_3D/Maletial/Material_GD/M_WallOverlap.M_WallOverlap")
    (`KismetSystemLibrary.Delay` 2.0)
    (`PrimitiveComponent.SetMaterial` (`self.DashWall`) 0 "/Game/Asset_3D/Maletial/Material_GD/M_DashEffect.M_DashEffect")))

(event `DashSetCollision`
  ;[0.4253 1 0.5549] Effet du Dash
  (`PrimitiveComponent.SetCollisionResponseToAllChannels` (`self.DashWall`) "ECR_Overlap")
  (`KismetSystemLibrary.Delay` (`self.TempsEffetDash(Sec)`))
  (`PrimitiveComponent.SetCollisionResponseToAllChannels` (`self.DashWall`) "ECR_Block"))

(fn `UserConstructionScript`)